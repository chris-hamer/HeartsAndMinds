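; Player controller that shows the mouse cursor and edge-scrolls a Camera pawn.
; Every tick it casts the controlled pawn to Camera, then compares the normalized mouse position with the outer tenth of the viewport on each side.
; Top and bottom edges drive MoveX and left and right edges drive MoveY with unit values, so corners trigger both axes.
; UI-only input mode and debug print nodes are left unconnected.
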(event EventBeginPlay
  (Variables|Default|SetbShowMouseCursor true))

(event EventTick
  (params (DeltaSeconds :type Float%20%28single-precision%29))
  (bind _returnvalue (Viewport|GetViewportSize))
  (bind (_locationx _locationy) (Game|Player|GetMousePosition))
  (bind (_x _y) (Math|Vector2D|BreakVector2D _returnvalue))
  (bind _returnvalue_2 (/ _locationy _y))
  (bind _returnvalue_3 (/ _locationx _x))
  (bind _ascamera (Utilities|Casting|CastToCamera (Pawn|GetControlledPawn)))
  (Variables|Default|SetCam _ascamera)
  (Utilities|FlowControl|Sequence
    (:then_0
      (if (< 0.9 _returnvalue_2)
        (Default|MoveX (Variables|Default|GetCam) -1.0)))
    (:then_1
      (if (< _returnvalue_3 0.1)
        (Default|MoveY (Variables|Default|GetCam) -1.0)))
    (:then_2
      (if (< _returnvalue_2 0.1)
        (Default|MoveX (Variables|Default|GetCam) 1.0)))
    (:then_3
      (if (< 0.9 _returnvalue_3)
        (Default|MoveY (Variables|Default|GetCam) 1.0)))))

(fn ConstructionScript)